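; Weapon pickup spawner that shows spinning, rapidly cycling random weapon meshes and grants a random weapon to the player or a GOAP enemy on overlap.
; Players get a reroll of any melee weapon already in their inventory, while enemies only receive ranged weapons.
; After pickup it hides, reactivates on a Tick-driven cooldown, then immediately serves an overlapping player first, otherwise an overlapping enemy.
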(event `self.ReceiveBeginPlay`
  (bind _outitem (`KismetArrayLibrary.Array_Random` (`self.PossibleWeapons`)))
  (`self.Display` (`.MeleeMesh` (break `WeaponDetails` _outitem)) (`.RangedMesh` (break `WeaponDetails` _outitem)))
  (bind _returnvalue (`GameplayStatics.GetActorOfClass` "/Script/DissProject.PlayerCharacter"))
  (set `self.Player` _returnvalue))

(event `self.ReceiveTick`
  (params (DeltaSeconds :type "Float (single-precision)"))
  (bind _player (`self.Player`))
  (bind _outitem (`KismetArrayLibrary.Array_Random` (`self.PossibleWeapons`)))
  (`SceneComponent.K2_AddLocalRotation` (`self.StaticMesh`) (struct :`Yaw` 2.0) false false)
  (`SceneComponent.K2_AddLocalRotation` (`self.SkeletalMesh`) (struct :`Yaw` 2.0) false false)
  (if (`self.Active`)
    (bind _output_get (set `self.RandomTimer` (+ (`self.RandomTimer`) DeltaSeconds)))
    (if (>= _output_get 0.4)
      (`self.Display` (`.MeleeMesh` (break `WeaponDetails` _outitem)) (`.RangedMesh` (break `WeaponDetails` _outitem)))
      (set `self.RandomTimer` 0.0))
    (else
      (bind _output_get_2 (set `self.ActiveTimer` (+ (`self.ActiveTimer`) DeltaSeconds)))
      (if (>= _output_get_2 20.0)
        (set `self.Active` true)
        (set `self.ActiveTimer` 0.0)
        (`|ExecutionSequence`
          (:`then_0`
            (if (`self.IsOverlappingActor` _player)
              (`self.Pickup` _player)
              (else
                (bind _outactors (`GameplayStatics.GetAllActorsOfClass` "/Script/DissProject.GOAPEnemy"))
                (for _array_element _outactors
                  (if (`self.IsOverlappingActor` _array_element)
                    (`self.Pickup` _array_element)
                    (break)))))))))))

(event `Display`
  (params (StaticMesh :type "StaticMesh Object Reference") (SkeletalMesh :type "SkeletalMesh Object Reference"))
  (bind _skeletalmesh (`self.SkeletalMesh`))
  (bind _staticmesh (`self.StaticMesh`))
  (`/Engine/EditorBlueprintResources/StandardMacros.IsValid` StaticMesh
    (:`Is Valid`
      (`StaticMeshComponent.SetStaticMesh` _staticmesh StaticMesh)
      (`SceneComponent.SetVisibility` _staticmesh true true)
      (`SceneComponent.SetVisibility` _skeletalmesh false true))
    (:`Is Not Valid`
      (`SkinnedMeshComponent.SetSkinnedAssetAndUpdate` _skeletalmesh SkeletalMesh true)
      (`SceneComponent.SetVisibility` _skeletalmesh true true)
      (`SceneComponent.SetVisibility` _staticmesh false true))))

(event `self.Sphere.OnComponentBeginOverlap`
  (params (OverlappedComponent :type "PrimitiveComponent Object Reference") (OtherActor :type "Actor Object Reference") (OtherComp :type "PrimitiveComponent Object Reference") (OtherBodyIndex :type Integer) (bFromSweep :type Boolean) (SweepResult :type "HitResult Structure (by ref)"))
  (bind _returnvalue (`GameplayStatics.GetObjectClass` OtherActor))
  (if (and (`self.Active`) (or (== _returnvalue "/Script/DissProject.PlayerCharacter") (== _returnvalue "/Script/DissProject.GOAPEnemy")))
    (`self.Pickup` OtherActor)))

(event `Pickup`
  (params (Actor :type "Actor Object Reference"))
  (bind _enemy (`self.Enemy`))
  (cast `PlayerCharacter` Actor
    (:`then`
      (set `self.Active` false)
      (`SceneComponent.SetVisibility` (`self.StaticMesh`) false true)
      (`SceneComponent.SetVisibility` (`self.SkeletalMesh`) false true)
      (bind _weapon (`self.ChooseWeapon` :!label _label))
      (if (!= (`.Name` (break `WeaponDetails` _weapon)) "None")
        (`PlayerCharacter.PickUp` (`self.Player`) _weapon 0)
        (else
          (goto _label))))
    (:`CastFailed`
      (bind _asgoapenemy (cast `GOAPEnemy` Actor))
      (set `self.Enemy` _asgoapenemy)
      (set `self.Active` false)
      (`SceneComponent.SetVisibility` (`self.StaticMesh`) false true)
      (`SceneComponent.SetVisibility` (`self.SkeletalMesh`) false true)
      (bind _output_get (set `self.Weapon` (`KismetArrayLibrary.Array_Random` (`self.PossibleWeapons`)) :!label _label_2))
      (if (`|EnumInequality` (`.Type` (break `WeaponDetails` _output_get)) "RANGED")
        (goto _label_2)
        (else
          (`GOAPEnemy.PickupWeapon` _enemy (`self.Weapon`) _enemy))))))

(fn `ChooseWeapon`
  (returns (Weapon :type "WeaponDetails Structure"))
  (locals (Found :type Boolean) (ChosenWeapon :type "WeaponDetails Structure") (ActorsInventory :type "Array of WeaponDetails Structure"))
  (set `local.ActorsInventory` (`Inventory.Inventory` (`PlayerCharacter.Inventory` (`self.Player`))))
  (bind _output_get (set `local.ChosenWeapon` (`KismetArrayLibrary.Array_Random` (`self.PossibleWeapons`)) :!label _label))
  (set `local.Found` false)
  (for _array_element (`local.ActorsInventory`)
    (if (== (break `WeaponDetails` _array_element) (break `WeaponDetails` _output_get))
      (if (`|EnumEquality` (`.Type` (break `WeaponDetails` _array_element)) "MELEE")
        (set `local.Found` true)
        (break))))
  (if (`local.Found`)
    (goto _label)
    (else
      (return (`local.ChosenWeapon`)))))

(fn `UserConstructionScript`)