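; BP_EnemySpawner spawns waves of GOAPEnemy actors in the level and signals when each wave has been wiped out.
; NewWave spawns enemies at random points inside the Box component's bounds until the requested count is reached, adjusting for collisions but always spawning.
; Each enemy's OnDeath feeds a death counter; when it matches the spawned count, both counters reset and the AllEnemiesDead dispatcher fires.
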(event `NewWave`
  (params (EnemiesToSpawn :type Integer))
  (while (< (`self.SpawnedEnemies`) EnemiesToSpawn)
    (`self.Spawn`)
    (`/Engine/EditorBlueprintResources/StandardMacros.IncrementInt` (`self.SpawnedEnemies`))))

(event `Spawn`
  (bind (_origin _boxextent) (`KismetSystemLibrary.GetComponentBounds` (`self.Box`)))
  (bind _returnvalue (`|SpawnActorFromClass` "/Script/DissProject.GOAPEnemy" (`KismetMathLibrary.MakeTransform` (`KismetMathLibrary.RandomPointInBoundingBox` _origin _boxextent)) "AdjustIfPossibleButAlwaysSpawn" "OverrideRootScale" null null))
  (add `GOAPEnemy.OnDeath` _returnvalue (delegate `OnDeath_Event_0`)))

(event `OnDeath_Event_0`
  (bind _result (`/Engine/EditorBlueprintResources/StandardMacros.IncrementInt` (`self.DeadEnemies`))
    (:`  `
      (if (== _result (`self.SpawnedEnemies`))
        (set `self.DeadEnemies` 0)
        (set `self.SpawnedEnemies` 0)
        (`self.AllEnemiesDead`)))))

(fn `UserConstructionScript`)