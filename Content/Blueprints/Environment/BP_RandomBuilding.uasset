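; BP_RandomBuilding is an environment actor that assembles a randomized building, either prebuilt or modular, when MakeBuilding is called.
; A percentage roll picks between a random prebuilt mesh and SpawnModularBuilding, which re-rolls until the entry matches the requested corner type.
; Modular entries set a base, then either add middle mesh components at stacked bounds-based heights for limitless types or set random middle and roof meshes, recording chosen meshes in Tiles.
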(fn `MakeBuilding`
  (params (IsCorner :type Boolean))
  (bind _base (`self.Base`))
  (if (< (`KismetMathLibrary.RandomIntegerInRange` 0 99) (`self.PercentChanceOfModular`))
    (`self.SpawnModularBuilding` IsCorner)
    (else
      (`StaticMeshComponent.SetStaticMesh` _base (`KismetArrayLibrary.Array_Random` (`self.PrebuildBuildings`)))
      (`KismetArrayLibrary.Array_Add` (`self.Tiles`) (`StaticMeshComponent.StaticMesh` _base)))))

(fn `SpawnModularBuilding`
  (params (IsCorner :type Boolean))
  (returns (Tiles :type "Array of StaticMesh Object Reference"))
  (locals (MidCounter :type Integer))
  (bind _middle (`self.Middle`))
  (bind _roof (`self.Roof`))
  (bind _output_get (set `self.Building` (`KismetArrayLibrary.Array_Random` (`self.ModularBuildings`)) :!label _label))
  (if (== IsCorner (`.IsCorner_12_CE48AEFA4A33C218AC8827A60329AD41` (break `/Game/StructsAndEnums/F_Building` _output_get)))
    (`StaticMeshComponent.SetStaticMesh` (`self.Base`) (break `/Game/StructsAndEnums/F_Building` _output_get))
    (`KismetArrayLibrary.Array_Add` (`self.Tiles`) (break `/Game/StructsAndEnums/F_Building` _output_get))
    (if (`.IsLimitless_10_FE32852844EE6B8121496AB7F9136E89` (break `/Game/StructsAndEnums/F_Building` _output_get))
      (bind _output_get_2 (set `self.MiddleTile` (`KismetArrayLibrary.Array_Random` (`.Middle_13_7A2912D34026FBA5D10C6DAFBCC7F766` (break `/Game/StructsAndEnums/F_Building` _output_get)))))
      (while (< (`local.MidCounter`) 5)
        (`AddComponent|NODE_AddStaticMeshComponent-0` :`RelativeTransform` (`KismetMathLibrary.MakeTransform` (`KismetMathLibrary.MakeVector` 0.0 0.0 (+ (* 2 (.z (`.BoxExtent` (`KismetMathLibrary.BreakBoxSphereBounds` (`StaticMesh.GetBounds` (`StaticMeshComponent.StaticMesh` (`self.Base`))))))) (* (* (`local.MidCounter`) 2) (.z (`.BoxExtent` (`KismetMathLibrary.BreakBoxSphereBounds` (`StaticMesh.GetBounds` _output_get_2))))))))))
      (else
        (`StaticMeshComponent.SetStaticMesh` _middle (`KismetArrayLibrary.Array_Random` (`.Middle_13_7A2912D34026FBA5D10C6DAFBCC7F766` (break `/Game/StructsAndEnums/F_Building` _output_get))))
        (`SceneComponent.K2_AddLocalOffset` _middle (`KismetMathLibrary.MakeVector` 0.0 0.0 (+ (* 2 (.z (`.BoxExtent` (`KismetMathLibrary.BreakBoxSphereBounds` (`StaticMesh.GetBounds` (`StaticMeshComponent.StaticMesh` _middle)))))) (* 2 (.z (`.BoxExtent` (`KismetMathLibrary.BreakBoxSphereBounds` (`StaticMesh.GetBounds` (`StaticMeshComponent.StaticMesh` (`self.Base`))))))))) false true)
        (`KismetArrayLibrary.Array_Add` (`self.Tiles`) (`StaticMeshComponent.StaticMesh` _middle))
        (`StaticMeshComponent.SetStaticMesh` _roof (`KismetArrayLibrary.Array_Random` (`.Roof_14_C86F85BE462006CA5D39B195B6EBE76A` (break `/Game/StructsAndEnums/F_Building` _output_get))))
        (`KismetArrayLibrary.Array_Add` (`self.Tiles`) (`StaticMeshComponent.StaticMesh` _roof))
        (return (`self.Tiles`))))
    (else
      (goto _label))))

(fn `UserConstructionScript`)