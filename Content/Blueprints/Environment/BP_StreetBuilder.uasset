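; Street builder actor that spawns a row of BP_RandomBuilding actors along the X or Y axis at BeginPlay.
; The construction script sizes a thin box to show the street's extent.
; Spawn loops space buildings by each mesh's X bounds plus a gap until the length is filled, with random yaw on Y streets.
; When a corner is required, the last building is replaced by a corner variant.
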(event `self.ReceiveBeginPlay`
  (`self.BuildStreet`))

(fn `BuildStreet`
  (locals (TotalLength :type "Float (double-precision)") (NewBuilding :type "/Game/Blueprints/Environment/BP_RandomBuilding Object Reference"))
  (switch `/Game/StructsAndEnums/EVertHori` (`self.Orientation`)
    (:`NewEnumerator1`
      (`self.X-Spawn`))
    (:`NewEnumerator0`
      (`self.Y_Spawn`))))

(fn `UserConstructionScript`
  (bind _streetlength (`self.StreetLength`))
  (bind _box (`self.Box`))
  (`BoxComponent.SetBoxExtent` _box (`KismetMathLibrary.MakeVector` _streetlength 0.001 0.001) false)
  (`SceneComponent.K2_SetRelativeLocation` _box (`KismetMathLibrary.MakeVector` _streetlength) false true))